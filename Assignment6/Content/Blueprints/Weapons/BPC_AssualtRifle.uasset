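; Assault rifle weapon Blueprint that fires a hitscan trace and sends damage to whatever it hits.
; WeaponTrace runs a camera trace to find the aim point, then sphere-traces from the muzzle Arrow toward it.
; Actors implementing BPI_Damage receive a Points value that rises with each consecutive hit and resets to zero on any other result.
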(event `self.WeaponTrace`
  (bind _returnvalue (`SceneComponent.K2_GetComponentLocation` (`self.Arrow`)))
  (bind (_newparam _outhits) (`/Game/Blueprints/Libraries/BPFL_Traces.Camera Trace` 8000.0))
  (bind _outhit (`KismetSystemLibrary.SphereTraceSingle` _returnvalue (+ (* (`KismetMathLibrary.GetForwardVector` (`KismetMathLibrary.FindLookAtRotation` _returnvalue (`.ImpactPoint` (`GameplayStatics.BreakHitResult` _outhits)))) 8000.0) _returnvalue) 1.0 "TraceTypeQuery1"))
  (bind (_bblockinghit _binitialoverlap _time _distance _location _impactpoint _normal _impactnormal _physmat _hitactor) (`GameplayStatics.BreakHitResult` _outhit))
  (if (`KismetSystemLibrary.DoesImplementInterface` _hitactor "/Game/Blueprints/Weapons/BPI_Damage.BPI_Damage_C")
    (bind _output_get (set `self.Points` (+ (`self.Points`) 1)))
    (message `/Game/Blueprints/Weapons/BPI_Damage.ReceiveDamage` _hitactor _output_get)
    (else
      (set `self.Points` 0))))

(fn `UserConstructionScript`
  (`parent.UserConstructionScript`))