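; BP_Target is a target actor that animates by a randomly chosen behavior and explodes when damaged.
; The construction script randomizes its scale and picks a TargetBehavior enum value.
; BeginPlay plays a timeline at a random rate, lerping the mesh horizontally or vertically by a random distance, or scaling it up.
; Damage spawns an explosion sound and particle effect at the mesh, then destroys the actor.
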(event `self.ReceiveBeginPlay`
  (bind _returnvalue (`KismetMathLibrary.RandomFloatInRange` 100.0 250.0))
  (bind _actorscale (`self.ActorScale`))
  (bind _returnvalue_2 (* _actorscale 1.5))
  (switch `/Game/Blueprints/Target/E_TargetBehavior` (`self.TargetBehavior`)
    (:`NewEnumerator1`
      (set `self.DestinationLocation` (`KismetMathLibrary.MakeVector` _returnvalue)))
    (:`NewEnumerator2`
      (set `self.DestinationLocation` (`KismetMathLibrary.MakeVector` 0.0 0.0 _returnvalue)))
    (:`NewEnumerator3`
      _))
  (`TimelineComponent.SetPlayRate` (`self.T_Move`) (/ 1.0 (`KismetMathLibrary.RandomFloatInRange` 1.5 3.0)))
  (bind (_direction _alpha) (`Timeline|T_Move` :!via `PlayFromStart`)
    (:`Update`
      (switch `/Game/Blueprints/Target/E_TargetBehavior` (`self.TargetBehavior`)
        (:`NewEnumerator1`
          (`SceneComponent.K2_SetRelativeLocation` (`self.StaticMesh`) (`KismetMathLibrary.VLerp` (0.0 0.0 0.0) (`self.DestinationLocation`) _alpha) false false :!label _label))
        (:`NewEnumerator2`
          (goto _label))
        (:`NewEnumerator3`
          (`SceneComponent.SetWorldScale3D` (`self.StaticMesh`) (`KismetMathLibrary.VLerp` (`KismetMathLibrary.MakeVector` _actorscale _actorscale _actorscale) (`KismetMathLibrary.MakeVector` _returnvalue_2 _returnvalue_2 _returnvalue_2) _alpha)))))))

(event `/Game/Blueprints/Weapons/BPI_Damage.ReceiveDamage`
  (bind _returnvalue (`SceneComponent.K2_GetComponentLocation` (`self.StaticMesh`)))
  (`GameplayStatics.SpawnSoundAtLocation` "/Game/StarterContent/Audio/Explosion_Cue.Explosion_Cue" _returnvalue (struct) 1.0 1.0 0.0 null null)
  (`GameplayStatics.SpawnEmitterAtLocation` "/Game/StarterContent/Particles/P_Explosion.P_Explosion" _returnvalue (struct) (0.2 0.2 0.2))
  (`self.K2_DestroyActor`))

(fn `UserConstructionScript`
  (bind _output_get (set `self.ActorScale` (`KismetMathLibrary.RandomFloatInRange` 0.25 1.0)))
  (`SceneComponent.SetWorldScale3D` (`self.DefaultSceneRoot`) (`KismetMathLibrary.MakeVector` _output_get _output_get _output_get))
  (set `self.TargetBehavior` (cast `/Game/Blueprints/Target/E_TargetBehavior` (`KismetMathLibrary.Conv_IntToByte` (`KismetMathLibrary.RandomIntegerInRange` 1 3)))))