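; Interactable push button that fires an Interact dispatcher when E is pressed while it is recently rendered, presumably for spawning logic bound elsewhere.
; An overlap area enables input, tick and a prompt text for the first-person character, with tick turning the text toward the camera.
; Each press plays a sound, while a DoOnce gates only the timeline that moves the button down.
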(event `self.ReceiveBeginPlay`
  (`SceneComponent.SetHiddenInGame` (`self.TextRender`) true false))

(event `Interacted`
  ;[1 1 1] Future useage
)

(event `Key|E`
  (params (Key :type "Key Structure"))
  (:`Pressed`
    (if (`self.WasRecentlyRendered` 0.2)
      (`self.Interacted`)
      (`self.Dispatch_Interact`)
      (`GameplayStatics.PlaySoundAtLocation` "/Game/StarterContent/Audio/Explosion01.Explosion01" (`SceneComponent.K2_GetComponentLocation` (`self.Button`)) (struct) 1.0 1.0 0.0 null null null null)
      (`/Engine/EditorBlueprintResources/StandardMacros.DoOnce` false :!label _label
        (:`Completed`
          (bind (_direction _alpha_value) (`Timeline|Animation` :!via `PlayFromStart`)
            (:`Update`
              (`SceneComponent.K2_SetRelativeLocation` (`self.Button`) (`KismetMathLibrary.VLerp` (0.0 0.0 0.0) (0.0 0.0 -10.0) _alpha_value) false false))
            (:`Finished`
              (goto _label :!via `Reset`))))))))

(event `self.C_Interaction_Area.OnComponentBeginOverlap`
  (params (OverlappedComponent :type "PrimitiveComponent Object Reference") (OtherActor :type "Actor Object Reference") (OtherComp :type "PrimitiveComponent Object Reference") (OtherBodyIndex :type Integer) (bFromSweep :type Boolean) (SweepResult :type "HitResult Structure (by ref)"))
  (cast `/Game/FirstPerson/Blueprints/BP_FirstPersonCharacter` OtherActor)
  (`self.EnableInput` (`GameplayStatics.GetPlayerController` 0))
  (`self.SetActorTickEnabled` true)
  (`SceneComponent.SetHiddenInGame` (`self.TextRender`) false false))

(event `self.C_Interaction_Area.OnComponentEndOverlap`
  (params (OverlappedComponent :type "PrimitiveComponent Object Reference") (OtherActor :type "Actor Object Reference") (OtherComp :type "PrimitiveComponent Object Reference") (OtherBodyIndex :type Integer))
  (cast `/Game/FirstPerson/Blueprints/BP_FirstPersonCharacter` OtherActor)
  (`self.DisableInput` (`GameplayStatics.GetPlayerController` 0))
  (`self.SetActorTickEnabled` false)
  (`SceneComponent.SetHiddenInGame` (`self.TextRender`) true false))

(event `self.ReceiveTick`
  (params (DeltaSeconds :type "Float (single-precision)"))
  (bind _textrender (`self.TextRender`))
  (`SceneComponent.K2_SetWorldRotation` _textrender (`KismetMathLibrary.FindLookAtRotation` (`SceneComponent.K2_GetComponentLocation` _textrender) (`SceneComponent.K2_GetComponentLocation` (`PlayerCameraManager.TransformComponent` (`GameplayStatics.GetPlayerCameraManager` 0)))) false false))

(fn `UserConstructionScript`)